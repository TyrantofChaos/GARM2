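; Base character Blueprint that equips a rifle and links it to health and animation through event dispatchers.
; On BeginPlay it spawns WeaponClass through a Child Actor Component, caches the rifle and anim Blueprint, then binds attack, hurt, death, reload and clip-change events.
; If either cast fails it prints an error and destroys itself.
; HandleDeath disables collision, triggers the death animation and notifies the weapon.
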(event `self.ReceiveBeginPlay`
  (bind _childactorcomponent (`self.ChildActorComponent`))
  ;[1 1 1] Comment
  (`parent.ReceiveBeginPlay`)
  (`ChildActorComponent.SetChildActorClass` _childactorcomponent (`self.WeaponClass`))
  (bind _asbp_base_rifle (cast `/Game/Blueprint/Actors/BP_BaseRifle` (`ChildActorComponent.ChildActor` _childactorcomponent))
    (:`then`
      (set `self.Weapon` _asbp_base_rifle)
      (bind _asabp_character_animation (cast `/Game/Both/ABP_CharacterAnimation` (`SkeletalMeshComponent.GetAnimInstance` (`self.Mesh`)))
        (:`then`
          (set `self.AnimBP` _asabp_character_animation)
          (add `/Game/Blueprint/Actors/BP_BaseRifle.OnRifleAttack` (`self.Weapon`) (`|CreateDelegate` (`self.AnimBP`) :!event `FireAnimation`))
          (add `/Game/Blueprint/Utility/AC_HealthComponent.OnHurt` (`self.AC_HealthComponent`) (`|CreateDelegate` (`self.AnimBP`) :!event `HitAnimation`))
          (add `/Game/Blueprint/Utility/AC_HealthComponent.OnDeath` (`self.AC_HealthComponent`) (`|CreateDelegate` :!event `HandleDeath`))
          (add `/Game/Blueprint/Actors/BP_BaseRifle.OnReloadStart` (`self.Weapon`) (`|CreateDelegate` (`self.AnimBP`) :!event `ReloadAnimation`))
          (add `/Game/Both/ABP_CharacterAnimation.OnReloadEnd` (`self.AnimBP`) (`|CreateDelegate` (`self.Weapon`) :!event `ActionStopped`))
          (add `/Game/Both/ABP_CharacterAnimation.OnClipChange` (`self.AnimBP`) (`|CreateDelegate` (`self.Weapon`) :!event `Reload Ammo`)))
        (:`CastFailed`
          (`KismetSystemLibrary.PrintString` "We do not have the correct animation")
          (`self.K2_DestroyActor`))))
    (:`CastFailed`
      (`KismetSystemLibrary.PrintString` "The Weapon is not set")
      (`self.K2_DestroyActor`))))

(fn `HandleDeath`
  (params (Ratio :type "Float (double-precision)"))
  (`self.SetActorEnableCollision` false)
  (`/Game/Both/ABP_CharacterAnimation.DeathAnimation` (`self.AnimBP`) Ratio)
  (`/Game/Blueprint/Actors/BP_BaseRifle.OwnerDied` (`self.Weapon`)))

(fn `UserConstructionScript`)
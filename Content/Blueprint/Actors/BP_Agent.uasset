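; BP_Agent is an AI-controlled combat agent that links its weapon and health component to its AI controller's brain.
; On begin play it tints its mesh, binds weapon-stopped and hurt events, and seeds the blackboard health ratio at full.
; Helpers send an action-ended AI message and write health ratio to the blackboard.
; Weapon attacks fire from EnemyAttack and also every Tick.
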(event `self.ReceiveBeginPlay`
  ;[1 1 1] Comment
  (`parent.ReceiveBeginPlay`)
  (`MeshComponent.SetVectorParameterValueOnMaterials` (`self.Mesh`) "Tint" (`KismetMathLibrary.Conv_LinearColorToVector` (`self.Color`)))
  (add `/Game/Blueprint/Actors/BP_BaseRifle.OnActionStopped` (`self.Weapon`) (`|CreateDelegate` :!event `HandleActionStopped`))
  (add `/Game/Blueprint/Utility/AC_HealthComponent.OnHurt` (`self.AC_HealthComponent`) (`|CreateDelegate` :!event `UpdateBlackboardHealth`))
  (`self.UpdateBlackboardHealth` 1.0))

(event `self.ReceiveTick`
  (params (DeltaSeconds :type "Float (single-precision)"))
  ;[1 1 1] Comment
  (`parent.ReceiveTick` DeltaSeconds)
  (`/Game/Blueprint/Actors/BP_BaseRifle.Attack` (`self.Weapon`)))

(event `/Game/Blueprint/Utility/BI_EnemyInterface.EnemyAttack`
  (`/Game/Blueprint/Actors/BP_BaseRifle.Attack` (`self.Weapon`)))

(fn `HandleActionStopped`
  (`AIBlueprintHelperLibrary.SendAIMessage` self (`self.Action Ended Message`)))

(fn `UpdateBlackboardHealth`
  (params (Ratio :type "Float (double-precision)"))
  (`BlackboardComponent.SetValueAsFloat` (`AIController.Blackboard` (`AIBlueprintHelperLibrary.GetAIController` self)) (`self.Health Ratio Name`) Ratio))

(fn `UserConstructionScript`
  (`parent.UserConstructionScript`))
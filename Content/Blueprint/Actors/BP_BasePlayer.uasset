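; Base player character Blueprint that handles movement, look and attack input, a viewport widget, and death.
; On BeginPlay it caches the PlayerController, creates and displays the WidgetClass widget, and binds to the health component's OnHurt and OnDeath events.
; Movement follows control yaw only, and the attack action delegates to the Weapon.
; The HandleDeath override calls the parent, then disables player input.
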(event `self.ReceiveBeginPlay`
  ;[1 1 1] Comment
  (`parent.ReceiveBeginPlay`)
  (bind _asplayer_controller (cast `PlayerController` (`self.GetController`))
    (:`then`
      (set `self.PlayerController` _asplayer_controller)
      (bind _returnvalue (`|CreateWidget` (`self.WidgetClass`) _asplayer_controller))
      (`UserWidget.AddToViewport` _returnvalue 0)
      (add `/Game/Blueprint/Utility/AC_HealthComponent.OnHurt` (`self.AC_HealthComponent`) (`|CreateDelegate` _returnvalue :!event `SetHealth`))
      (add `/Game/Blueprint/Utility/AC_HealthComponent.OnDeath` (`self.AC_HealthComponent`) (`|CreateDelegate` _returnvalue :!event `SetHealth`)))
    (:`CastFailed`
      (`KismetSystemLibrary.PrintString` "No Contorller"))))

(event `InputAxis|TurnRight`
  (params (AxisValue :type "Float (single-precision)"))
  ;[1 1 1] Comment
  ;;[1 1 1] Comment
  (`self.AddControllerYawInput` AxisValue))

(event `InputAxis|LookUp`
  (params (AxisValue :type "Float (single-precision)"))
  ;[1 1 1] Comment
  (`self.AddControllerPitchInput` AxisValue))

(event `InputAxis|MoveForward`
  (params (AxisValue :type "Float (single-precision)"))
  ;[1 1 1] Comment
  ;;[1 1 1] Doing the binding for you
  (`self.AddMovementInput` (`KismetMathLibrary.GetForwardVector` (`KismetMathLibrary.MakeRotator` 0.0 0.0 (.yaw (`self.GetControlRotation`)))) AxisValue))

(event `InputAxis|Strafe`
  (params (AxisValue :type "Float (single-precision)"))
  ;[1 1 1] Comment
  (`self.AddMovementInput` (`KismetMathLibrary.GetRightVector` (`KismetMathLibrary.MakeRotator` 0.0 0.0 (.yaw (`self.GetControlRotation`)))) AxisValue))

(event `InputAction|AttackInput`
  (params (Key :type "Key Structure"))
  ;[1 1 1] Comment
  (:`Pressed`
    (`/Game/Blueprint/Actors/BP_BaseRifle.Attack` (`self.Weapon`))))

(fn `HandleDeath`
  (params (Ratio :type "Float (double-precision)"))
  (`parent.HandleDeath` Ratio)
  (`self.DisableInput` (`self.PlayerController`)))

(fn `UserConstructionScript`
  (`parent.UserConstructionScript`))
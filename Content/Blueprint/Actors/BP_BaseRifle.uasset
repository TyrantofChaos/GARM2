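; BP_BaseRifle is a base rifle actor that fires projectiles for the pawn it is parented to, destroying itself if that parent is not a pawn.
; Attack is blocked while an action runs or after owner death, spawns the projectile at a mesh socket, and starts a two-second timer.
; A Blueprint-only hack aims player shots at the HUD widget's destination, while other pawns use base aim rotation.
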(event `self.ReceiveBeginPlay`
  ;[1 1 1] Comment
  (`parent.ReceiveBeginPlay`)
  (bind _aspawn (cast `Pawn` (`self.GetParentActor`))
    (:`then`
      (set `self.ParentPawn` _aspawn))
    (:`CastFailed`
      (`KismetSystemLibrary.PrintString` "We need to be owned by a pawn")
      (`self.K2_DestroyActor`))))

(event `OwnerDied`
  (set `self.OwnerAlive` false))

(event `ActionStopped`
  ;[1 1 1] Comment
  (set `self.ActionHappening` false)
  (`self.OnActionStopped`))

(fn `Attack`
  (bind _parentpawn (`self.ParentPawn`))
  ;[1 1 1] Comment
  (if (`self.CanAttack`)
    (`|SpawnActorFromClass` (`self.ProjectileClass`) (`KismetMathLibrary.MakeTransform` (`self.GetSource`) (`self.HACK_DO_NOT_PUT_IN_CODE`)) "Undefined" "MultiplyWithRoot" (`Pawn.GetController` _parentpawn) _parentpawn)
    (set `self.ActionHappening` true)
    (`KismetSystemLibrary.K2_SetTimerDelegate` (`|CreateDelegate` :!event `ActionStopped`) 2.0)
    (`self.OnRifleAttack`)))

(fn `CanAttack`
  (returns (Yes :type Boolean))
  ;[1 1 1] Comment
  (return (and (not (`self.ActionHappening`)) (`self.OwnerAlive`))))

(fn `GetSource`
  (returns (ReturnValue :type "Vector Structure"))
  (return (`SceneComponent.GetSocketLocation` (`self.SkeletalMesh`) (`self.SocketName`))))

(fn `HACK_DO_NOT_PUT_IN_CODE`
  (returns (Rotation :type "Rotator Structure"))
  ;[1 1 1] Blueprint Only - Test to see if Parent pawn is the player
  (bind _foundwidgets (`WidgetBlueprintLibrary.GetAllWidgetsOfClass` "/Game/Both/WBP_PlayerHUD.WBP_PlayerHUD_C" false))
  (bind _output (`|GetArrayItem` _foundwidgets))
  (if (== (`UserWidget.GetOwningPlayerPawn` _output) (`self.ParentPawn`))
    ;[1 1 1] This is the code that will be in the player override of Get base aim roation
    (return (`KismetMathLibrary.MakeRotFromX` (- (`/Game/Both/WBP_PlayerHUD.GetDestination` _output) (`self.GetSource`))))
    (else
      ;[1 1 1] This is  the AI do nothing different
      (return (`Pawn.GetBaseAimRotation` (`self.ParentPawn`))))))

(fn `UserConstructionScript`)
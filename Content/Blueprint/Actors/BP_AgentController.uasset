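; BP_AgentController is an AI controller that runs a behavior tree when it possesses a pawn.
; The construction script binds the AI Perception component's target-update event to a perception handler.
; The handler stores a successfully sensed actor in the blackboard under the player key and clears that key when sensing fails.
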(event `self.ReceivePossess`
  (params (PossessedPawn :type "Pawn Object Reference"))
  (`parent.ReceivePossess` null)
  (`self.RunBehaviorTree` (`self.BTAsset`)))

(fn `Handle Perception`
  (params (Actor :type "Actor Object Reference") (Stimulus :type "AIStimulus Structure"))
  (if (`.bSuccessfullySensed` (break `AIStimulus` Stimulus))
    (`BlackboardComponent.SetValueAsObject` (`self.Blackboard`) (`self.Player Key`) Actor)
    (else
      (`BlackboardComponent.ClearValue` (`self.Blackboard`) (`self.Player Key`)))))

(fn `UserConstructionScript`
  (add `AIPerceptionComponent.OnTargetPerceptionUpdated` (`self.AIPerception`) (`|CreateDelegate` :!event `Handle Perception`)))
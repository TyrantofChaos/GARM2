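; Game Instance Blueprint that provides level loading and a quit action for the game.
; LoadFirstLevel passes FirstLevelIndex to LoadLevelSafe, which validates the index against the GameLevels array before opening that level by name.
; An invalid index prints an error message pointing to the array instead of opening a level.
; A separate QuitGame event exits the application.
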(event `LoadFirstLevel`
  (`self.LoadLevelSafe` (`self.FirstLevelIndex`)))

(event `QuitGame`
  (`KismetSystemLibrary.QuitGame` null "Quit"))

(fn `LoadLevelSafe`
  (params (`Dimension 1` :type Integer))
  (bind _gamelevels (`self.GameLevels`))
  (if (`KismetArrayLibrary.Array_IsValidIndex` _gamelevels `Dimension 1`)
    (`GameplayStatics.OpenLevel` (`|GetArrayItem` _gamelevels `Dimension 1`))
    (else
      (`KismetSystemLibrary.PrintString` (`KismetStringLibrary.Concat_StrStr` "Could Not Load Level index: " (`KismetStringLibrary.Conv_IntToString` `Dimension 1`) " Check your Array")))))